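; BP_MovingTarget is a destructible target that travels along a spline path taken from a referenced Path actor at BeginPlay.
; Each tick advances a distance by MoveSpeed and teleports the actor to that point on the spline, wrapping to the start past the end.
; Damage lowers Health, and at zero it notifies GameMode_BP through MovingTargetWasDestroyed before destroying itself.
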(event EventBeginPlay
  (Variables|Default|SetSpline (Variables|/Game/Blueprint/Ennemis/BP_Path.BP_Path_C|GetPath (Variables|Components|GetPath))))

(event Collision|EventActorBeginOverlap
  (params (OtherActor :type Actor%20Object%20Reference)))

(event EventTick
  (params (DeltaSeconds :type Float%20%28single-precision%29))
  (bind _spline (Variables|Default|GetSpline))
  (bind _returnvalue (Spline|GetSplineLength _spline))
  (bind _output_get (Variables|Default|SetDistance (+ (Variables|Default|GetDistance) (* (Variables|Default|GetMoveSpeed) DeltaSeconds))))
  (if (< _output_get _returnvalue)
    (bind _output_get_2 (Variables|Default|SetTargetLocation (Spline|GetLocationatDistanceAlongSpline (Variables|Default|GetSpline) (stale _output_get_3) "World")))
    (Transformation|SetActorLocation _output_get_2 false false)
    (else
      (bind _output_get_3 (Variables|Default|SetDistance (- (Variables|Default|GetDistance) _returnvalue))))))

(event Game|Damage|EventAnyDamage
  (params (Damage :type Float%20%28single-precision%29) (DamageType :type Damage%20Type%20Object%20Reference) (InstigatedBy :type Controller%20Object%20Reference) (DamageCauser :type Actor%20Object%20Reference))
  (CallFunction|TakeDamage Damage))

(fn ConstructionScript)

(fn TakeDamage
  (params (Damage :type Float%20%28single-precision%29))
  (bind _output_get (Variables|Default|SetHealth (- (Variables|Default|GetHealth) Damage)))
  (if (<= _output_get 0.0)
    (bind _asgame_mode_bp (Utilities|Casting|CastToGameMode_BP (Game|GetGameMode)))
    (Default|MovingTargetWasDestroyed _asgame_mode_bp self)
    (Actor|DestroyActor)))