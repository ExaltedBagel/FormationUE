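; GameMode_BP is a game mode that tracks how many moving and static targets remain in the level.
; On BeginPlay it gathers all BP_MovingTarget and BP_StaticTarget actors into two arrays.
; Destruction events for each type remove the actor from its array, then UpdateRemainingTargets writes the combined count to the Remaining text on the player character's HUD.
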(event Custom|StaticWasDestroyed
  (params (DestroyedActor :type Actor%20Object%20Reference))
  (bind _asbp_static_target (Utilities|Casting|CastToBP_StaticTarget DestroyedActor))
  (Utilities|Array|RemoveItem (Variables|Default|GetStaticTargets) _asbp_static_target)
  (CallFunction|UpdateRemainingTargets))

(event Custom|MovingTargetWasDestroyed
  (params (DestroyedActor :type Actor%20Object%20Reference))
  (bind _asbp_moving_target (Utilities|Casting|CastToBP_MovingTarget DestroyedActor))
  (Utilities|Array|RemoveItem (Variables|Default|GetMovingTargets) _asbp_moving_target)
  (CallFunction|UpdateRemainingTargets))

(event EventBeginPlay
  (bind _outactors (Actor|GetAllActorsOfClass "/Game/Blueprint/Ennemis/BP_MovingTarget.BP_MovingTarget_C"))
  (Variables|Default|SetMovingTargets _outactors)
  (bind _outactors_2 (Actor|GetAllActorsOfClass "/Game/Blueprint/Ennemis/BP_StaticTarget.BP_StaticTarget_C"))
  (Variables|Default|SetStaticTargets _outactors_2)
  (CallFunction|UpdateRemainingTargets))

(event EventTick
  (params (DeltaSeconds :type Float%20%28single-precision%29)))

(fn ConstructionScript)

(fn UpdateRemainingTargets
  (bind _asplayer_character_bp (Utilities|Casting|CastToPlayerCharacter_BP (Game|GetPlayerCharacter 0)))
  (Rendering|Components|TextRender|SetText (Variables|/Game/Blueprint/BP_HUD.BP_HUD_C|GetRemaining (Variables|/Game/Blueprint/Player/PlayerCharacter_BP.PlayerCharacter_BP_C|GetHUD _asplayer_character_bp)) (Utilities|Text|MakeLiteralText (Utilities|Text|ToText(String) (Utilities|String|Append "Remaining: " (Utilities|String|ToString(Integer) (+ (Utilities|Array|Length (Variables|Default|GetMovingTargets)) (Utilities|Array|Length (Variables|Default|GetStaticTargets)))))))))